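; Forest chest actor (Orman2) that opens when the third-person character enters its trigger box and shows the Konum_orman2 location widget.
; Begin overlap enables input and creates the widget if the chest is still closed; end overlap disables input and removes it.
; Tick polls the trigger and plays the OpenChest timeline to rotate the lid's roll, guarded by IsOpen and IsMoving.
; The CloseChest logic is disconnected, so the chest stays open.
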(event `self.TriggerBox.OnComponentBeginOverlap`
  (params (OverlappedComponent :type "PrimitiveComponent Object Reference") (OtherActor :type "Actor Object Reference") (OtherComp :type "PrimitiveComponent Object Reference") (OtherBodyIndex :type Integer) (bFromSweep :type Boolean) (SweepResult :type "HitResult Structure (by ref)"))
  (cast `/Game/ThirdPerson/Blueprints/BP_ThirdPersonCharacter` OtherActor)
  (`self.EnableInput` (`GameplayStatics.GetPlayerController` 0))
  (if (not (`self.isOpen`))
    (bind _returnvalue (`|CreateWidget` "/Game/Widget/konum_orman2.konum_orman2_C"))
    (`UserWidget.AddToViewport` _returnvalue 0)))

(event `self.ReceiveTick`
  (params (DeltaSeconds :type "Float (single-precision)"))
  (if (`self.isMoving`)
    _
    (elif (> (`KismetArrayLibrary.Array_Length` (`PrimitiveComponent.GetOverlappingActors` (`self.TriggerBox`) "/Game/ThirdPerson/Blueprints/BP_ThirdPersonCharacter.BP_ThirdPersonCharacter_C")) 0)
      (if (not (`self.isOpen`))
        (set `self.isMoving` true)
        (bind (_direction _chestangle) (`Timeline|OpenChest` :!via `PlayFromStart`)
          (:`Update`
            (`SceneComponent.K2_SetRelativeRotation` (`self.SandikKapak`) (`KismetMathLibrary.MakeRotator` _chestangle) false false)
            (set `self.isOpen` true)
            (set `self.isMoving` false)))))))

(event `self.TriggerBox.OnComponentEndOverlap`
  (params (OverlappedComponent :type "PrimitiveComponent Object Reference") (OtherActor :type "Actor Object Reference") (OtherComp :type "PrimitiveComponent Object Reference") (OtherBodyIndex :type Integer))
  (cast `/Game/ThirdPerson/Blueprints/BP_ThirdPersonCharacter` OtherActor)
  (`self.DisableInput` (`GameplayStatics.GetPlayerController` 0))
  (`Widget.RemoveFromParent` (stale `self.TriggerBox.OnComponentBeginOverlap` _returnvalue)))

(fn `UserConstructionScript`)