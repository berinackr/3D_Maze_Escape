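; Chest Blueprint that lights up and swings its lid open when the third-person character enters its trigger box.
; Entering reveals the Spott component on a closed chest and enables actor input, which leaving disables.
; Tick polls the trigger's overlaps and plays the OpenChest timeline to rotate the SandikKapak lid on roll, latching IsOpen so it stays open.
; Closing, timer and FirstChest widget logic is present but disconnected.
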(event `self.TriggerBox.OnComponentBeginOverlap`
  (params (OverlappedComponent :type "PrimitiveComponent Object Reference") (OtherActor :type "Actor Object Reference") (OtherComp :type "PrimitiveComponent Object Reference") (OtherBodyIndex :type Integer) (bFromSweep :type Boolean) (SweepResult :type "HitResult Structure (by ref)"))
  (cast `/Game/ThirdPerson/Blueprints/BP_ThirdPersonCharacter` OtherActor)
  (`self.EnableInput` (`GameplayStatics.GetPlayerController` 0))
  (if (not (`self.isOpen`))
    (`SceneComponent.SetVisibility` (`self.spott`) true false)))

(event `self.ReceiveTick`
  (params (DeltaSeconds :type "Float (single-precision)"))
  (if (`self.isMoving`)
    _
    (elif (> (`KismetArrayLibrary.Array_Length` (`PrimitiveComponent.GetOverlappingActors` (`self.TriggerBox`) "/Game/ThirdPerson/Blueprints/BP_ThirdPersonCharacter.BP_ThirdPersonCharacter_C")) 0)
      (if (not (`self.isOpen`))
        (set `self.isMoving` true)
        (bind (_direction _chestangle) (`Timeline|OpenChest` :!via `PlayFromStart`)
          (:`Update`
            (`SceneComponent.K2_SetRelativeRotation` (`self.SandikKapak`) (`KismetMathLibrary.MakeRotator` _chestangle) false false)
            (set `self.isOpen` true)
            (set `self.isMoving` false)))))))

(event `self.TriggerBox.OnComponentEndOverlap`
  (params (OverlappedComponent :type "PrimitiveComponent Object Reference") (OtherActor :type "Actor Object Reference") (OtherComp :type "PrimitiveComponent Object Reference") (OtherBodyIndex :type Integer))
  (cast `/Game/ThirdPerson/Blueprints/BP_ThirdPersonCharacter` OtherActor)
  (`self.DisableInput` (`GameplayStatics.GetPlayerController` 0)))

(fn `UserConstructionScript`)